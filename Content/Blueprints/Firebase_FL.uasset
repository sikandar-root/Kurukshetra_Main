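; Firebase function library for user status and lobby presence data in the database.
; Two helpers build database references to the Status and Lobby nodes under each user's Profile, keyed by UID.
; A parser reads a lobby snapshot's value as a map and, when the IsInLobby key exists, returns that flag with the LobbyID.
; Validate is an empty stub.
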(fn StatusPath
  (params (UID :type String))
  (return (Class|FGDatabaseRef|Child (Class|FGDatabaseRef|Child (Class|FGDatabaseRef|Child (Class|FGDatabaseRef|MakeDatabaseReffromPath "users") UID) "Profile") "Status")))

(fn LobbyStatusPath
  (params (UID :type String))
  (return (Class|FGDatabaseRef|Child (Class|FGDatabaseRef|Child (Class|FGDatabaseRef|Child (Class|FGDatabaseRef|MakeDatabaseReffromPath "users") UID) "Profile") "Lobby")))

(fn GetLobbyStatusValue
  (params (Data :type FG%20Data%20Snapshot%20Object%20Reference))
  (bind _returnvalue (Class|FGDataSnapshot|GetValue Data))
  (if (.ReturnValue (Utilities|Map|Find (Class|FGValueVariantAccess|GetMap _returnvalue) "IsInLobby"))
    (return (Class|FGValueVariantAccess|GetBool (.Value (Utilities|Map|Find (Class|FGValueVariantAccess|GetMap _returnvalue) "IsInLobby"))) (Class|FGValueVariantAccess|GetInteger (.Value (Utilities|Map|Find (Class|FGValueVariantAccess|GetMap _returnvalue) "LobbyID"))))))

(fn Validate)